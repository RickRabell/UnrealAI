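; Crossing signal actor that cycles between Green, Yellow and Red to tell Smart Object users whether to cross, be aware or wait.
; StateTree state-change events dispatch by gameplay tag to handlers, starting Green on BeginPlay.
; Handlers swap the Activities.CrossPath tag on the first slot of two Smart Objects and recolor an emissive sphere.
; Construction sizes the collision box; HandleYellow and HandleRed are uncalled single-object variants.
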(event Custom|HandleStateChange
  (params (State :type Gameplay%20Tag%20Structure))
  (|SwitchGameplayTag State
    (:Default
      (Development|PrintString "Failed to Dispatch State"))
    (:State.Green
      (CallFunction|HandleGreen))
    (:State.Yellow
      (CallFunction|HandleYellowness))
    (:State.Red
      (CallFunction|HandleRednesss))))

(event EventBeginPlay
  (Development|PrintString (Utilities|String|EnumtoString (Class|StateTreeComponent|GetStateTreeRunStatus (Variables|Default|GetStateTree))))
  (EventDispatchers|BindEventtoOnNewState (EventDispatchers|CreateEvent :!event Custom|HandleStateChange))
  (CallFunction|HandleGreen))

(event Collision|EventActorBeginOverlap
  (params (OtherActor :type Actor%20Object%20Reference)))

(event EventTick
  (params (DeltaSeconds :type Float%20%28single-precision%29)))

(fn ConstructionScript
  (Components|Box|SetBoxExtent (Variables|Default|GetCrossCollision) (Math|Vector|MakeVector (Variables|Default|GetCrossWidth) (Variables|Default|GetCrossLength) (Variables|Default|GetCrossHeight)) true))

(fn HandleGreen
  (bind _returnvalue (GameplayTags|MakeLiteralGameplayTag "(TagName=\"Activities.CrossPath.Cross\")"))
  (bind _returnvalue_2 (Subsystems|GetSmartObjectSubsystem))
  (bind _returnvalue_3 (Subsystems|GetSmartObjectSubsystem))
  (bind _smartobjectcross2 (Variables|Default|GetSmartObjectCross2))
  (bind _smartobjectcross (Variables|Default|GetSmartObjectCross))
  (bind _registeredhandle (Variables|/Script/SmartObjectsModule.SmartObjectComponent|GetRegisteredHandle _smartobjectcross2))
  (bind _registeredhandle_2 (Variables|/Script/SmartObjectsModule.SmartObjectComponent|GetRegisteredHandle _smartobjectcross))
  (bind _outslots (Class|SmartObjectSubsystem|GetAllSlots _returnvalue_3 _registeredhandle_2))
  (bind _outslots_2 (Class|SmartObjectSubsystem|GetAllSlots _returnvalue_2 _registeredhandle))
  (bind _output (Utilities|Array|Get(acopy) _outslots))
  (bind _output_2 (Utilities|Array|Get(acopy) _outslots_2))
  (Class|SmartObjectSubsystem|RemoveTagfromSlot _returnvalue_3 _output (Variables|Default|GetLastState))
  (Class|SmartObjectSubsystem|AddTagtoSlot _returnvalue_3 _output _returnvalue)
  (Class|SmartObjectSubsystem|RemoveTagfromSlot _returnvalue_2 _output_2 (Variables|Default|GetLastState))
  (Class|SmartObjectSubsystem|AddTagtoSlot _returnvalue_2 _output_2 _returnvalue)
  (Variables|Default|SetLastState _returnvalue)
  (bind _returnvalue_4 (Rendering|Material|CreateDynamicMaterialInstance (Variables|Default|GetSphere) 0 0 "None" :!class /Script/Engine.PrimitiveComponent))
  (Rendering|Material|SetVectorParameterValue _returnvalue_4 "Emissive Color" "(R=0.099329,G=1.000000,B=0.007506,A=1.000000)" :!class /Script/Engine.MaterialInstanceDynamic)
  (Development|PrintString (GameplayTags|GetDebugStringfromGameplayTag (Variables|Default|GetLastState))))

(fn HandleYellow
  (bind _returnvalue (GameplayTags|MakeLiteralGameplayTag "(TagName=\"Activities.CrossPath.Aware\")"))
  (bind _returnvalue_2 (Subsystems|GetSmartObjectSubsystem))
  (bind _smartobjectcross (Variables|Default|GetSmartObjectCross))
  (bind _registeredhandle (Variables|/Script/SmartObjectsModule.SmartObjectComponent|GetRegisteredHandle _smartobjectcross))
  (bind _outslots (Class|SmartObjectSubsystem|GetAllSlots _returnvalue_2 _registeredhandle))
  (bind _output (Utilities|Array|Get(acopy) _outslots))
  (Class|SmartObjectSubsystem|RemoveTagfromSlot _returnvalue_2 _output (Variables|Default|GetLastState))
  (Class|SmartObjectSubsystem|AddTagtoSlot _returnvalue_2 _output _returnvalue)
  (Variables|Default|SetLastState _returnvalue)
  (bind _returnvalue_3 (Rendering|Material|CreateDynamicMaterialInstance (Variables|Default|GetSphere) 0 0 "None" :!class /Script/Engine.PrimitiveComponent))
  (Rendering|Material|SetVectorParameterValue _returnvalue_3 "Emissive Color" "(R=0.977431,G=0.788452,B=0.110300,A=1.000000)" :!class /Script/Engine.MaterialInstanceDynamic)
  (Development|PrintString (GameplayTags|GetDebugStringfromGameplayTag (Variables|Default|GetLastState))))

(fn HandleRed
  (bind _returnvalue (GameplayTags|MakeLiteralGameplayTag "(TagName=\"Activities.CrossPath.Wait\")"))
  (bind _returnvalue_2 (Subsystems|GetSmartObjectSubsystem))
  (bind _smartobjectcross (Variables|Default|GetSmartObjectCross))
  (bind _registeredhandle (Variables|/Script/SmartObjectsModule.SmartObjectComponent|GetRegisteredHandle _smartobjectcross))
  (bind _outslots (Class|SmartObjectSubsystem|GetAllSlots _returnvalue_2 _registeredhandle))
  (bind _output (Utilities|Array|Get(acopy) _outslots))
  (Class|SmartObjectSubsystem|RemoveTagfromSlot _returnvalue_2 _output (Variables|Default|GetLastState))
  (Class|SmartObjectSubsystem|AddTagtoSlot _returnvalue_2 _output _returnvalue)
  (Variables|Default|SetLastState _returnvalue)
  (bind _returnvalue_3 (Rendering|Material|CreateDynamicMaterialInstance (Variables|Default|GetSphere) 0 0 "None" :!class /Script/Engine.PrimitiveComponent))
  (Rendering|Material|SetVectorParameterValue _returnvalue_3 "Emissive Color" "(R=0.824653,G=0.004240,B=0.000000,A=1.000000)" :!class /Script/Engine.MaterialInstanceDynamic)
  (Development|PrintString (GameplayTags|GetDebugStringfromGameplayTag (Variables|Default|GetLastState))))

(fn HandleYellowness
  (bind _returnvalue (GameplayTags|MakeLiteralGameplayTag "(TagName=\"Activities.CrossPath.Aware\")"))
  (bind _returnvalue_2 (Subsystems|GetSmartObjectSubsystem))
  (bind _returnvalue_3 (Subsystems|GetSmartObjectSubsystem))
  (bind _smartobjectcross2 (Variables|Default|GetSmartObjectCross2))
  (bind _smartobjectcross (Variables|Default|GetSmartObjectCross))
  (bind _registeredhandle (Variables|/Script/SmartObjectsModule.SmartObjectComponent|GetRegisteredHandle _smartobjectcross2))
  (bind _registeredhandle_2 (Variables|/Script/SmartObjectsModule.SmartObjectComponent|GetRegisteredHandle _smartobjectcross))
  (bind _outslots (Class|SmartObjectSubsystem|GetAllSlots _returnvalue_3 _registeredhandle_2))
  (bind _outslots_2 (Class|SmartObjectSubsystem|GetAllSlots _returnvalue_2 _registeredhandle))
  (bind _output (Utilities|Array|Get(acopy) _outslots))
  (bind _output_2 (Utilities|Array|Get(acopy) _outslots_2))
  (Class|SmartObjectSubsystem|RemoveTagfromSlot _returnvalue_3 _output (Variables|Default|GetLastState))
  (Class|SmartObjectSubsystem|AddTagtoSlot _returnvalue_3 _output _returnvalue)
  (Class|SmartObjectSubsystem|RemoveTagfromSlot _returnvalue_2 _output_2 (Variables|Default|GetLastState))
  (Class|SmartObjectSubsystem|AddTagtoSlot _returnvalue_2 _output_2 _returnvalue)
  (Variables|Default|SetLastState _returnvalue)
  (bind _returnvalue_4 (Rendering|Material|CreateDynamicMaterialInstance (Variables|Default|GetSphere) 0 0 "None" :!class /Script/Engine.PrimitiveComponent))
  (Rendering|Material|SetVectorParameterValue _returnvalue_4 "Emissive Color" "(R=0.977431,G=0.788452,B=0.110300,A=1.000000)" :!class /Script/Engine.MaterialInstanceDynamic)
  (Development|PrintString (GameplayTags|GetDebugStringfromGameplayTag (Variables|Default|GetLastState))))

(fn HandleRednesss
  (bind _returnvalue (GameplayTags|MakeLiteralGameplayTag "(TagName=\"Activities.CrossPath.Wait\")"))
  (bind _returnvalue_2 (Subsystems|GetSmartObjectSubsystem))
  (bind _returnvalue_3 (Subsystems|GetSmartObjectSubsystem))
  (bind _smartobjectcross2 (Variables|Default|GetSmartObjectCross2))
  (bind _smartobjectcross (Variables|Default|GetSmartObjectCross))
  (bind _registeredhandle (Variables|/Script/SmartObjectsModule.SmartObjectComponent|GetRegisteredHandle _smartobjectcross2))
  (bind _registeredhandle_2 (Variables|/Script/SmartObjectsModule.SmartObjectComponent|GetRegisteredHandle _smartobjectcross))
  (bind _outslots (Class|SmartObjectSubsystem|GetAllSlots _returnvalue_3 _registeredhandle_2))
  (bind _outslots_2 (Class|SmartObjectSubsystem|GetAllSlots _returnvalue_2 _registeredhandle))
  (bind _output (Utilities|Array|Get(acopy) _outslots))
  (bind _output_2 (Utilities|Array|Get(acopy) _outslots_2))
  (Class|SmartObjectSubsystem|RemoveTagfromSlot _returnvalue_3 _output (Variables|Default|GetLastState))
  (Class|SmartObjectSubsystem|AddTagtoSlot _returnvalue_3 _output _returnvalue)
  (Class|SmartObjectSubsystem|RemoveTagfromSlot _returnvalue_2 _output_2 (Variables|Default|GetLastState))
  (Class|SmartObjectSubsystem|AddTagtoSlot _returnvalue_2 _output_2 _returnvalue)
  (Variables|Default|SetLastState _returnvalue)
  (bind _returnvalue_4 (Rendering|Material|CreateDynamicMaterialInstance (Variables|Default|GetSphere) 0 0 "None" :!class /Script/Engine.PrimitiveComponent))
  (Rendering|Material|SetVectorParameterValue _returnvalue_4 "Emissive Color" "(R=0.824653,G=0.004240,B=0.000000,A=1.000000)" :!class /Script/Engine.MaterialInstanceDynamic)
  (Development|PrintString (GameplayTags|GetDebugStringfromGameplayTag (Variables|Default|GetLastState))))